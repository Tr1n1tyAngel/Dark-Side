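; BP_OxygenTank is an oxygen pickup that the first-person character collects by touching it.
; On BeginPlay it stores the point light's starting intensity, then plays the LightFlash timeline, which scales that intensity to flash the light.
; When BP_FirstPersonCharacter overlaps the capsule, the tank calls that character's OxygenIncrease and destroys itself.
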(event `self.ReceiveBeginPlay`
  (set `self.StartIntensity` (`LightComponentBase.Intensity` (`self.PointLight`)))
  (bind (_direction _flashintensity) (`Timeline|LightFlash`)
    (:`Update`
      (`LightComponent.SetIntensity` (`self.PointLight`) (* _flashintensity (`self.StartIntensity`))))))

(event `self.Capsule.OnComponentBeginOverlap`
  (params (OverlappedComponent :type "PrimitiveComponent Object Reference") (OtherActor :type "Actor Object Reference") (OtherComp :type "PrimitiveComponent Object Reference") (OtherBodyIndex :type Integer) (bFromSweep :type Boolean) (SweepResult :type "HitResult Structure (by ref)"))
  (bind _asbp_first_person_character (cast `/Game/MainGame/Blueprints/BP_FirstPersonCharacter` OtherActor))
  (`/Game/MainGame/Blueprints/BP_FirstPersonCharacter.OxygenIncrease` _asbp_first_person_character)
  (`self.K2_DestroyActor`))

(fn `UserConstructionScript`)