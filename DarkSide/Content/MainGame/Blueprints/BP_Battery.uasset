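; BP_Battery is a battery pickup that either of two local players can collect.
; On spawn it plays a ping sound and a LightFlash timeline scales its point light from the starting intensity.
; Overlapping its collision matches the actor to player 0 or 1, each with its own character class, calls BatteryIncrease on that character and destroys the pickup.
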(event `self.ReceiveBeginPlay`
  (`GameplayStatics.PlaySoundAtLocation` "/Game/MainGame/MusicSFX/ItemPing.ItemPing" (`self.K2_GetActorLocation` self) (struct) 0.025 0.5 0.0 null null null null)
  (set `self.StartIntensity` (`LightComponentBase.Intensity` (`self.PointLight`)))
  (bind (_direction _flashintensity) (`Timeline|LightFlash`)
    (:`Update`
      (`LightComponent.SetIntensity` (`self.PointLight`) (* _flashintensity (`self.StartIntensity`))))))

(event `self.Collision.OnComponentBeginOverlap`
  (params (OverlappedComponent :type "PrimitiveComponent Object Reference") (OtherActor :type "Actor Object Reference") (OtherComp :type "PrimitiveComponent Object Reference") (OtherBodyIndex :type Integer) (bFromSweep :type Boolean) (SweepResult :type "HitResult Structure (by ref)"))
  (bind _returnvalue (`GameplayStatics.GetPlayerCharacter` 0))
  (bind _returnvalue_2 (`GameplayStatics.GetPlayerCharacter` 1))
  (if (== OtherActor _returnvalue)
    (bind _asbp_first_person_character (cast `/Game/MainGame/Blueprints/BP_FirstPersonCharacter` _returnvalue))
    (`/Game/MainGame/Blueprints/BP_FirstPersonCharacter.BatteryIncrease` _asbp_first_person_character)
    (`self.K2_DestroyActor` :!label _label)
    (elif (== OtherActor _returnvalue_2)
      (bind _asbp_first_person_character_1 (cast `/Game/MainGame/Blueprints/BP_FirstPersonCharacter1` _returnvalue_2))
      (`/Game/MainGame/Blueprints/BP_FirstPersonCharacter1.BatteryIncrease` _asbp_first_person_character_1)
      (goto _label))))

(fn `UserConstructionScript`)