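; Key is a collectible pickup that adds to the KeysFound count of whichever of two players touches it.
; When its Box is overlapped, it checks the other actor against player characters 0 and 1.
; Each player is cast to its own class, BP_FirstPersonCharacter or BP_FirstPersonCharacter1, to increment that character's counter.
; The key then destroys itself, and other overlapping actors are ignored.
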(event `self.Box.OnComponentBeginOverlap`
  (params (OverlappedComponent :type "PrimitiveComponent Object Reference") (OtherActor :type "Actor Object Reference") (OtherComp :type "PrimitiveComponent Object Reference") (OtherBodyIndex :type Integer) (bFromSweep :type Boolean) (SweepResult :type "HitResult Structure (by ref)"))
  (bind _returnvalue (`GameplayStatics.GetPlayerCharacter` 0))
  (bind _returnvalue_2 (`GameplayStatics.GetPlayerCharacter` 1))
  (if (== OtherActor _returnvalue)
    (bind _asbp_first_person_character (cast `/Game/MainGame/Blueprints/BP_FirstPersonCharacter` _returnvalue))
    (bind _result (`/Engine/EditorBlueprintResources/StandardMacros.IncrementInt` (`/Game/MainGame/Blueprints/BP_FirstPersonCharacter.KeysFound` _asbp_first_person_character))
      (:`  `
        (set `/Game/MainGame/Blueprints/BP_FirstPersonCharacter.KeysFound` _result _asbp_first_person_character)
        (`self.K2_DestroyActor` :!label _label)))
    (elif (== OtherActor _returnvalue_2)
      (bind _asbp_first_person_character_1 (cast `/Game/MainGame/Blueprints/BP_FirstPersonCharacter1` _returnvalue_2))
      (bind _result_2 (`/Engine/EditorBlueprintResources/StandardMacros.IncrementInt` (`/Game/MainGame/Blueprints/BP_FirstPersonCharacter1.KeysFound` _asbp_first_person_character_1))
        (:`  `
          (set `/Game/MainGame/Blueprints/BP_FirstPersonCharacter1.KeysFound` _result_2 _asbp_first_person_character_1)
          (goto _label))))))

(fn `UserConstructionScript`)